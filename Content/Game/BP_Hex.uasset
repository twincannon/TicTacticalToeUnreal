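; BP_Hex is a hex tile actor that shows ownership and capturable state on its mesh.
; Construction creates a dynamic material instance from the neutral material.
; SetOwnership and SetCapturable call their parent versions, then respectively swap in the player, opponent or neutral material and set the "Capturable" scalar parameter on the mesh materials.
; SetDebugText writes row and column to a text render; OnMouseOver is empty.
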(event `self.SetCapturable`
  (params (bIsCapturable :type Boolean))
  (`parent.SetCapturable` bIsCapturable)
  (`MeshComponent.SetScalarParameterValueOnMaterials` (`self.HexMesh`) "Capturable" (`KismetMathLibrary.Conv_BoolToDouble` bIsCapturable)))

(event `self.OnMouseOver`
  (params (Actor :type "Actor Object Reference")))

(event `self.SetOwnership`
  (params (Player :type "EPlayerType Enum" :default "PLAYER"))
  (`parent.SetOwnership` Player)
  (`PrimitiveComponent.SetMaterial` (`self.HexMesh`) 0 (select `EPlayerType` Player :`PLAYER` "/Game/Assets/Materials/M_Hex_Player.M_Hex_Player" :`OPPONENT` "/Game/Assets/Materials/M_Hex_Opponent.M_Hex_Opponent" :`NEUTRAL` "/Game/Assets/Materials/M_Hex_Neutral.M_Hex_Neutral" :!type "MaterialInterface Object Reference")))

(event `self.SetDebugText`
  (params (Row :type Integer) (Col :type Integer))
  (`TextRenderComponent.K2_SetText` (`self.TextRender`) (`|FormatText` "{0},{1}" Row Col)))

(fn `UserConstructionScript`
  (`PrimitiveComponent.CreateDynamicMaterialInstance` (`self.HexMesh`) 0 "/Game/Assets/Materials/M_Hex_Neutral.M_Hex_Neutral" "None"))