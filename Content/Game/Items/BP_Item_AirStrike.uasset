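; Item Blueprint for an air strike that clears a row or column of the tic-tac-toe board from a player-selected center wall tile.
; On execute it puts the GameState into item tile-selection mode and binds to the tile-selected event.
; A successful clear on the Board marks the item used, ends selection and passes the turn; a failed clear leaves selection active.
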(event `self.ExecuteItem`
  (params (GameState :type "TacGameState Object Reference"))
  (`TacGameState.SetSelectingTileForItem` GameState true)
  (add `TacGameState.OnItemTileSelected` GameState (delegate `TileSelected`))
  (set `self.GameState` GameState))

(event `TileSelected`
  (params (SelectedTile :type "TacBoardTile Object Reference"))
  (bind _gamestate (`self.GameState`))
  (bind _returnvalue (`TacBoard.ClearRowOrColFromCenterWallTile` (`TacGameState.Board` (`self.GameState`)) SelectedTile))
  (if _returnvalue
    (`self.OnItemUsed`)
    (`TacGameState.SetSelectingTileForItem` _gamestate false)
    (`TacGameState.PassTicTacToeTurn` _gamestate)))