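; BP_Item_APC is a usable item for a tic-tac-toe style board game.
; On use it fills up to two random empty board tiles with the offensive team's mark, OH for the player and EX otherwise.
; It checks for game over after each placement, passes the turn only while the game continues, and always signals that the item was used.
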(event `self.ExecuteItem`
  (params (GameState :type "TacGameState Object Reference"))
  (bind _returnvalue (select `bool` (`|EnumEquality` (`TacGameState.OffensiveTeam` GameState) "PLAYER") :`false` "EX" :`true` "OH" :!type "ETileType Enum"))
  (bind _returnvalue_2 (`TacBoard.GetRandomEmptyTile` (`TacGameState.Board` GameState)))
  (`TacBoardTile.SetTileType` _returnvalue_2 _returnvalue)
  (if (not (`TacGameState.IsBoardGameOver` GameState))
    (bind _returnvalue_3 (`TacBoard.GetRandomEmptyTile` (`TacGameState.Board` GameState)))
    (`TacBoardTile.SetTileType` _returnvalue_3 _returnvalue)
    (if (not (`TacGameState.IsBoardGameOver` GameState))
      (`TacGameState.PassTicTacToeTurn` GameState)))
  (`self.OnItemUsed`))