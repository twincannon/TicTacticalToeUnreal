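; BP_Item_Missile is a usable item in a tic-tac-toe game that clears a 3x3 area of the board around a chosen tile.
; On execute it puts the GameState into item tile-selection mode, binds to its tile-selected event and makes every board tile selectable.
; Once a tile is picked, it empties the surrounding tiles, signals that the item was used, exits selection mode and passes the turn.
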(event `self.ExecuteItem`
  (params (GameState :type "TacGameState Object Reference"))
  (`TacGameState.SetSelectingTileForItem` GameState true)
  (clear `TacGameState.OnItemTileSelected` GameState)
  (add `TacGameState.OnItemTileSelected` GameState (delegate `TileSelected`))
  (set `self.GameState` GameState)
  (bind _board (`TacGameState.Board` GameState)
    (:`then`
      (for _array_element (`TacBoard.TileRows` _board)
        (for _array_element_2 (`.TileCol` (break `TileArray` _array_element))
          (`TacBoardTile.SetTileSelectable` _array_element_2 true))))
    (:`else`)))

(event `TileSelected`
  (params (SelectedTile :type "TacBoardTile Object Reference"))
  (bind _gamestate (`self.GameState`))
  (bind _gamestate_2 (`self.GameState`))
  (bind _board (`TacGameState.Board` _gamestate_2))
  (clear `TacGameState.OnItemTileSelected` _gamestate_2)
  (for _array_element (`TacBoard.GetTilesIn3By3Radius` _board SelectedTile)
    (`TacBoardTile.SetTileType` _array_element "EMPTY"))
  (`self.OnItemUsed`)
  (`TacGameState.SetSelectingTileForItem` _gamestate false)
  (`TacGameState.PassTicTacToeTurn` _gamestate)
  (`TacBoard.ClearSelectableTiles` _board))