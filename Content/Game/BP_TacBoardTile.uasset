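; BP_TacBoardTile is a tic-tac-toe board tile that shows its current mark on a Plane component.
; SetTileType calls the parent implementation, then swaps the plane's material by tile type: O, X, or the same M_Trans material for empty and radioactive.
; A debug text path that labels each type with a letter remains in the graph but never runs.
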(event `self.SetTileType`
  (params (NewType :type "ETileType Enum" :default "EMPTY"))
  (`parent.SetTileType` NewType)
  (`PrimitiveComponent.SetMaterial` (`self.Plane`) 0 (select `ETileType` NewType :`EMPTY` "/Game/Assets/Materials/M_Trans.M_Trans" :`OH` "/Game/Assets/Materials/M_ttt_o.M_ttt_o" :`EX` "/Game/Assets/Materials/M_ttt_x.M_ttt_x" :`RADIOACTIVE` "/Game/Assets/Materials/M_Trans.M_Trans" :!type "MaterialInterface Object Reference")))

(fn `UserConstructionScript`)